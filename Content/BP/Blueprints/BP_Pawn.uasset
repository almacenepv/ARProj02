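; Player pawn for an ARCore image-hunt quiz, where characters found on tracked images ask questions that award trophies.
; It loads or creates the save on BeginPlay, then on Tick spawns one BP_Encanto per recognized image name, customized from DT_Encantos by splitting that name.
; A pinch while scanning line-traces for a character and opens its question through GlobalMenu.
; Correct answers update and async-save the trophy and call the character's Puf; misses show failure notifications.
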(event `self.ReceiveBeginPlay`
  ;[1 1 1] Iniciar y cargar partida
  (bind _returnvalue (`GameplayStatics.CreateSaveGameObject` "/Game/BP/Blueprints/BP_SaveGame.BP_SaveGame_C"))
  (bind _output_get (set `self.SaveGameInstance` _returnvalue))
  (bind _slot (`/Game/BP/Blueprints/BP_SaveGame.Slot` _output_get))
  (bind _index (`/Game/BP/Blueprints/BP_SaveGame.Index` _output_get))
  (bind _returnvalue_2 (`GameplayStatics.DoesSaveGameExist` _slot _index))
  (if (not _returnvalue_2)
    (`GameplayStatics.SaveGameToSlot` _output_get _slot _index))
  (bind _returnvalue_3 (`GameplayStatics.LoadGameFromSlot` _slot _index))
  (bind _asbp_save_game (cast `/Game/BP/Blueprints/BP_SaveGame` _returnvalue_3)
    (:`then`
      (set `self.SaveGameInstance` _asbp_save_game)
      (`KismetSystemLibrary.Delay` 0.2)
      (`self.PartidaCargada`))
    (:`CastFailed`
      (`KismetSystemLibrary.PrintString` "Error recuperando partida" true true (struct :`R` 1.0 :`B` 0.07339 :`A` 1.0) 25.0))))

(event `self.ReceiveTick`
  (params (DeltaSeconds :type "Float (single-precision)"))
  ;[1 1 1] Búsqueda y detección de imágenes trackeadas
  ;;[1 1 1] Configuración ARCore - Buscar imágenes trackeadas
  (bind _returnvalue (`ARBlueprintLibrary.GetAllGeometriesByClass` "/Script/GoogleARCoreBase.GoogleARCoreAugmentedImage"))
  (for _array_element _returnvalue
    (bind _returnvalue_2 (`GoogleARCoreAugmentedImage.GetImageName` _array_element))
    ;[1 1 1] Comprueba Etiqueta válida
    (if (`BlueprintMapLibrary.Map_Contains` (`self.TrofeosTemp`) _returnvalue_2)
      ;[1 1 1] Comprueba si el personaje ya ha sido generado y actualiza, si no es así
      (if (not (`KismetArrayLibrary.Array_Contains` (`self.SpawnedCharac`) _returnvalue_2))
        (`KismetArrayLibrary.Array_AddUnique` (`self.SpawnedCharac`) _returnvalue_2)
        ;[1 1 1] Spawn y particularización del personaje
        (bind _returnvalue_3 (`|SpawnActorFromClass` "/Game/Characters/BP_Encanto.BP_Encanto_C" (`ARTrackedGeometry.GetLocalToWorldTransform` _array_element) "Undefined" "OverrideRootScale" null null))
        (bind _output_get (set `self.ARCharac` _returnvalue_3))
        (`self.CustomizeEncanto` _output_get _returnvalue_2)))))

(event `Key|Gesture_Pinch`
  (params (Key :type "Key Structure"))
  (bind (_locationx _locationy) (`PlayerController.GetInputTouchState` (`GameplayStatics.GetPlayerController` 0) "Touch1"))
  ;[1 1 1] Plantear pregunta al jugador
  (:`Pressed`
    (if (`self.Scanning`)
      (bind (_outhit _returnvalue) (`self.HitCheck` (`KismetMathLibrary.MakeVector2D` _locationx _locationy)))
      (if _returnvalue
        (bind _asbp_encanto (cast `/Game/Characters/BP_Encanto` (`.HitActor` (`GameplayStatics.BreakHitResult` _outhit))))
        (bind _output_get (set `self.ARCharac` _asbp_encanto))
        (`/Game/UI/BP_Menu.AskQuestion` (`self.GlobalMenu`) (`/Game/Characters/BP_Encanto.ImageName` _output_get) _output_get)
        (else
          (`TextBlock.SetText` (`/Game/UI/BP_Notification.TextNotificacion` (`/Game/UI/BP_Menu.BP_Notificacion` (`self.GlobalMenu`))) "¡Apunta \nMejor!")
          (`/Game/UI/BP_Menu.NotiFail` (`self.GlobalMenu`)))))))

(event `RespuestaOK`
  ;[1 1 1] Plantear pregunta al jugador
  ;;[1 1 1] Respuesta Correcta - Trofeo
  (bind (_bp_trofeos _outputpin _textotrofeo _iconotrofeo _savegameinstance _slot _index) (`self.ActExtrac`))
  (bind (_icono _trofeotexto) (`/Game/UI/BP_Trophies.GetTrophyData` _bp_trofeos _outputpin))
  (`TextBlock.SetText` _textotrofeo _trofeotexto)
  (`Image.SetBrushTintColor` _iconotrofeo (make `SlateColor` (struct :`R` 1.0 :`G` 1.0 :`B` 1.0 :`A` 1.0)))
  (bind (_savegame _bsuccess) (`AsyncActionHandleSaveGame.AsyncSaveGameToSlot` _savegameinstance _slot _index)
    (:`then`
      (`/Game/Characters/BP_Encanto.Puf` (`self.ARCharac`)))
    (:`Completed`
      (if (not _bsuccess)
        (`KismetSystemLibrary.PrintString` "Error guardando")))))

(event `CompararRespuesta`
  ;[1 1 1] Plantear pregunta al jugador
  ;;[1 1 1] Evaluar respuesta recibida
  (if (`KismetTextLibrary.EqualEqual_TextText` (`self.RespuestaCorrecta`) (`self.RespuestaRecibida`))
    (`self.RespuestaOK`)
    (else
      (`self.RespuestaKO`))))

(event `RespuestaKO`
  ;[1 1 1] Plantear pregunta al jugador
  ;;[1 1 1] Respuesta Errónea - Mensaje
  (`TextBlock.SetText` (`/Game/UI/BP_Notification.TextNotificacion` (`/Game/UI/BP_Menu.BP_Notificacion` (`self.GlobalMenu`))) "¡¡¡Craso \nError!!!")
  (`/Game/UI/BP_Menu.NotiFail` (`self.GlobalMenu`)))

(fn `CustomizeEncanto`
  (params (Encanto :type "/Game/Characters/BP_Encanto Object Reference") (ImageName :type String))
  (bind (_lefts _rights) (`KismetStringLibrary.Split` ImageName "_"))
  (bind _encanto (`local.Encanto`))
  (bind _returnvalue (`KismetStringLibrary.Conv_StringToInt` _rights))
  (bind _skeletalmesh (`/Game/Characters/BP_Encanto.SkeletalMesh` (`local.Encanto`)))
  ;[1 1 1] Personalizar Encanto
  (set `/Game/Characters/BP_Encanto.Pawn` self (`local.Encanto`))
  (set `/Game/Characters/BP_Encanto.ImageName` ImageName (`local.Encanto`))
  (set `/Game/Characters/BP_Encanto.EncantoType` (`KismetStringLibrary.Conv_StringToName` _lefts) (`local.Encanto`))
  (set `/Game/Characters/BP_Encanto.Ubicacion` _returnvalue _encanto)
  (bind _returnvalue_2 (`|GetDataTableRow` "/Game/LocalData/DT_Encantos.DT_Encantos" (`/Game/Characters/BP_Encanto.EncantoType` _encanto))
    (:`then`
      (`SkinnedMeshComponent.SetSkinnedAssetAndUpdate` _skeletalmesh (break `/Game/LocalData/Struct_Encantos` _returnvalue_2) true)
      (`SkeletalMeshComponent.SetAnimation` _skeletalmesh (`.Anim_8_FD4511804C0AF885D0087F99B7E2BABA` (break `/Game/LocalData/Struct_Encantos` _returnvalue_2)))
      (`SkeletalMeshComponent.Play` _skeletalmesh true)
      (`self.InfoGlobo` (`local.Encanto`) (select `int` _returnvalue :`0` (`.Info1_9_0F24696047BB9E789ADF2D9A0BA5C9C7` (break `/Game/LocalData/Struct_Encantos` _returnvalue_2)) :`1` (`.Info2_13_32773F4441965206FB0F30859E12AAA8` (break `/Game/LocalData/Struct_Encantos` _returnvalue_2)) :`2` (`.Info3_14_3B57532B489B1982E432F898E485980B` (break `/Game/LocalData/Struct_Encantos` _returnvalue_2)) :`3` (`.Info4_15_FD4DBEC04030343C17C6BCBD2B4DFE0E` (break `/Game/LocalData/Struct_Encantos` _returnvalue_2))))
      (`self.EncantoPersonalizado`))))

(fn `HitCheck`
  (params (ScreenPosition :type "Vector2D Structure (by ref)"))
  (returns (OutHit :type "HitResult Structure") (ReturnValue :type Boolean))
  (bind (_worldposition _worlddirection) (`GameplayStatics.DeprojectScreenToWorld` (`GameplayStatics.GetPlayerController` 0) ScreenPosition))
  ;[1 1 1] Comprobación de hit
  (bind (_outhit _returnvalue) (`KismetSystemLibrary.LineTraceSingleForObjects` _worldposition (+ _worlddirection (* _worlddirection 1000.0)) (`|MakeArray` "ObjectTypeQuery1" "ObjectTypeQuery2" "ObjectTypeQuery3" "ObjectTypeQuery4" "ObjectTypeQuery5" "ObjectTypeQuery6" :!type "EObjectTypeQuery Enum")))
  (return _outhit _returnvalue))

(fn `InfoGlobo`
  (params (Encanto :type "/Game/Characters/BP_Encanto Object Reference") (Speech :type Text))
  ;[1 1 1] Actualizar info globo
  (`TextRenderComponent.K2_SetText` (`/Game/Characters/BP_Encanto.TextBubble` (`local.Encanto`)) Speech)
  (`TextRenderComponent.K2_SetText` (`/Game/Characters/BP_Encanto.TextBubbleBack` (`local.Encanto`)) Speech))

(fn `UserConstructionScript`)
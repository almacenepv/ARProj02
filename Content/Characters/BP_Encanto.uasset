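; BP_Encanto is a character actor that appears with a Niagara burst when the player pawn fires its custom Encanto event.
; On start it shows and activates two Niagara effects, yaws its root toward the pawn's camera, then reveals the skeletal mesh after a short delay.
; Puf replays the main effect, hides the mesh, speech bubble and shadow, then destroys the actor after the burst.
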(event `self.ReceiveBeginPlay`
  ;[1 1 1] BeginPlay
  (add `/Game/BP/Blueprints/BP_Pawn.EncantoPersonalizado` (cast `/Game/BP/Blueprints/BP_Pawn` (`GameplayStatics.GetPlayerPawn` 0) :!pure true) (delegate `Iniciar`)))

(event `Iniciar`
  (bind _niagara (`self.Niagara`))
  (bind _defaultsceneroot (`self.DefaultSceneRoot`))
  (bind (_returnvalue_roll _returnvalue_pitch) (`KismetMathLibrary.BreakRotator` (`SceneComponent.K2_GetComponentRotation` _defaultsceneroot)))
  (bind (_returnvalue_roll_2 _returnvalue_pitch_2 _returnvalue_yaw) (`KismetMathLibrary.BreakRotator` (`KismetMathLibrary.FindLookAtRotation` (`SceneComponent.K2_GetComponentLocation` _defaultsceneroot) (`SceneComponent.K2_GetComponentLocation` (`/Game/BP/Blueprints/BP_Pawn.Camera` (`self.Pawn`))))))
  ;[1 1 1] Iniciar: Visibilidad, mirar a cámara, explosión
  (`SceneComponent.SetVisibility` _niagara true false)
  (`SceneComponent.SetVisibility` (`self.NiagaraTop`) true false)
  (`ActorComponent.Activate` _niagara true)
  (`ActorComponent.Activate` (`self.NiagaraTop`) true)
  (`SceneComponent.K2_SetWorldRotation` _defaultsceneroot (`KismetMathLibrary.MakeRotator` _returnvalue_roll _returnvalue_pitch (- _returnvalue_yaw 90.0)) false false)
  (`KismetSystemLibrary.Delay` 2.0)
  (`SceneComponent.SetVisibility` (`self.SkeletalMesh`) true true))

(event `Puf`
  ;[1 1 1] Explosión final y captura
  (`NiagaraComponent.ResetSystem` (`self.Niagara`))
  (`SceneComponent.SetVisibility` (`self.SkeletalMesh`) false false)
  (`SceneComponent.SetVisibility` (`self.PlaneBubble`) false false)
  (`SceneComponent.SetVisibility` (`self.TextBubble`) false false)
  (`SceneComponent.SetVisibility` (`self.TextBubbleBack`) false false)
  (`SceneComponent.SetVisibility` (`self.Shadow`) false false)
  (`KismetSystemLibrary.Delay` 5.0)
  (`self.K2_DestroyActor`))

(fn `UserConstructionScript`)